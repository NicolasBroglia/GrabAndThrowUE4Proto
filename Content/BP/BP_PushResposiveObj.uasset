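; BP_PushResposiveObj is an actor whose mesh can be knocked away from a given point by an applied force.
; ApplyForce enables physics on the mesh and adds a mass-independent impulse along the direction away from the origin, scaled by Power.
; ResetForce_1 stops any active simulation, moves the actor to the mesh's location and detaches DefaultSceneRoot, while an unconnected attach node never runs.
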(event Custom|ResetForce_1
  (bind _mesh (Variables|Default|GetMesh))
  (if (Physics|IsSimulatingPhysics _mesh "None")
    (Physics|SetSimulatePhysics _mesh false)
    (Transformation|SetActorLocation (Transformation|GetWorldLocation _mesh) false false)
    (Transformation|DetachFromComponent (Variables|Default|GetDefaultSceneRoot) "KeepRelative" "KeepRelative" "KeepRelative" true)))

(event EventBeginPlay)

(event Collision|EventActorBeginOverlap
  (params (OtherActor :type Actor%20Object%20Reference)))

(event EventTick
  (params (DeltaSeconds :type Float%20%28single-precision%29)))

(event EventApplyForce
  (params (Force%20Origin :type Vector :default "0, 0, 0") (Power :type Float%20%28single-precision%29))
  (bind _mesh (Variables|Default|GetMesh))
  (Physics|SetSimulatePhysics _mesh true)
  (Physics|AddImpulse _mesh (* (Math|Vector|Normalize (- (Transformation|GetWorldLocation (Variables|Default|GetMesh)) Force%20Origin)) Power) "None" true))

(fn ConstructionScript)